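; Game mode that drives the time loop and its day-to-midnight lighting mood.
; Tick advances the TimeLoop object and periodically records the player pawn's location to the Ghosts object until midnight.
; TimeLoop events for loop start, approaching midnight and midnight set sun, color, skylight and fog targets.
; Tick eases the level's lights and height fog toward these targets, while ApplyTimeOfDay sets given values instantly.
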(event Custom|ApplyTimeOfDay
  (params (LightIntensity :type Float%20%28single-precision%29) (LightColor :type Linear%20Color%20Structure) (SkyIntensity :type Float%20%28single-precision%29) (FogDensity :type Float%20%28single-precision%29))
  (bind _returnvalue (Actor|GetActorOfClass "/Script/Engine.DirectionalLight"))
  (Rendering|Components|Light|SetIntensity (Actor|GetComponentbyClass _returnvalue "/Script/Engine.DirectionalLightComponent") LightIntensity)
  (Rendering|Components|Light|SetLightColor (Actor|GetComponentbyClass _returnvalue "/Script/Engine.DirectionalLightComponent") LightColor true)
  (bind _returnvalue_2 (Actor|GetActorOfClass "/Script/Engine.SkyLight"))
  (Rendering|Components|Light|SetIntensity (Actor|GetComponentbyClass _returnvalue_2 "/Script/Engine.SkyLightComponent") SkyIntensity)
  (bind _returnvalue_3 (Actor|GetActorOfClass "/Script/Engine.ExponentialHeightFog"))
  (Class|ExponentialHeightFogComponent|SetFogDensity (Actor|GetComponentbyClass _returnvalue_3 "/Script/Engine.ExponentialHeightFogComponent") FogDensity))

(event Custom|HandleMidnightApproaching
  (CallFunction|SetTimeOfDayTargets 0.9 "(R=1.0,G=0.55,B=0.3,A=1.0)" 0.5 0.03))

(event Custom|HandleMidnightTriggered
  (CallFunction|SetTimeOfDayTargets 0.04 "(R=0.35,G=0.45,B=0.9,A=1.0)" 0.1 0.08))

(event Custom|HandleLoopStarted
  (params (LoopNumber :type Integer))
  (CallFunction|SetTimeOfDayTargets 3.0 "(R=1.0,G=0.95,B=0.9,A=1.0)" 1.0 0.015))

(event EventTick
  (params (DeltaSeconds :type Float%20%28single-precision%29))
  (bind _timeloop (CallFunction|GetTimeLoop))
  (if (Utilities|IsValid _timeloop)
    (Default|AdvanceTime _timeloop DeltaSeconds)
    (Utilities|FlowControl|Sequence
      (:then_0
        (bind _output_get (Variables|Default|SetSampleAccum (+ (Variables|Default|GetSampleAccum) DeltaSeconds)))
        (if (>= _output_get 5.0)
          (Variables|Default|SetSampleAccum 0.0)
          (if (not (Variables|/Game/TVV/Blueprints/Core/Subsystems/BPS_TimeLoopSubsystem.BPS_TimeLoopSubsystem_C|GetbIsAfterMidnight _timeloop))
            (bind _ghosts (CallFunction|GetGhosts))
            (Default|RecordPoint _ghosts (Transformation|GetActorLocation (Game|Player|GetPlayerPawn 0))))))
      (:then_1
        (bind _returnvalue (Actor|GetActorOfClass "/Script/Engine.DirectionalLight"))
        (Rendering|Components|Light|SetIntensity (Actor|GetComponentbyClass _returnvalue "/Script/Engine.DirectionalLightComponent") (Math|Interpolation|FInterpTo (Variables|/Script/Engine.LightComponentBase|GetIntensity (Actor|GetComponentbyClass _returnvalue "/Script/Engine.DirectionalLightComponent")) (Variables|Default|GetTgtSun) DeltaSeconds 0.8))
        (Rendering|Components|Light|SetLightColor (Actor|GetComponentbyClass _returnvalue "/Script/Engine.DirectionalLightComponent") (Class|KismetMathLibrary|CInterpto (Math|Conversions|ToLinearColor(Color) (Variables|/Script/Engine.LightComponentBase|GetLightColor (Actor|GetComponentbyClass _returnvalue "/Script/Engine.DirectionalLightComponent"))) (Variables|Default|GetTgtColor) DeltaSeconds 0.8) true)
        (bind _returnvalue_2 (Actor|GetActorOfClass "/Script/Engine.SkyLight"))
        (Rendering|Components|Light|SetIntensity (Actor|GetComponentbyClass _returnvalue_2 "/Script/Engine.SkyLightComponent") (Math|Interpolation|FInterpTo (Variables|/Script/Engine.LightComponentBase|GetIntensity (Actor|GetComponentbyClass _returnvalue_2 "/Script/Engine.SkyLightComponent")) (Variables|Default|GetTgtSky) DeltaSeconds 0.8))
        (bind _returnvalue_3 (Actor|GetActorOfClass "/Script/Engine.ExponentialHeightFog"))
        (Class|ExponentialHeightFogComponent|SetFogDensity (Actor|GetComponentbyClass _returnvalue_3 "/Script/Engine.ExponentialHeightFogComponent") (Math|Interpolation|FInterpTo (Variables|/Script/Engine.ExponentialHeightFogComponent|GetFogDensity (Actor|GetComponentbyClass _returnvalue_3 "/Script/Engine.ExponentialHeightFogComponent")) (Variables|Default|GetTgtFog) DeltaSeconds 0.8))))))

(event EventBeginPlay
  (bind _timeloop (CallFunction|GetTimeLoop))
  (EventDispatchers|BindEventtoOnMidnightApproaching _timeloop (delegate Custom|HandleMidnightApproaching))
  (EventDispatchers|BindEventtoOnMidnightTriggered _timeloop (delegate Custom|HandleMidnightTriggered))
  (EventDispatchers|BindEventtoOnLoopStarted _timeloop (delegate Custom|HandleLoopStarted)))

(fn ConstructionScript)

(fn SetTimeOfDayTargets
  (params (Sun :type Float%20%28single-precision%29) (Color :type Linear%20Color%20Structure) (Sky :type Float%20%28single-precision%29) (Fog :type Float%20%28single-precision%29))
  (Variables|Default|SetTgtSun Sun)
  (Variables|Default|SetTgtColor Color)
  (Variables|Default|SetTgtSky Sky)
  (Variables|Default|SetTgtFog Fog))