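; AC_Mirror is an actor component that lets its owner use a mirror to flip the time era.
; UseMirror checks that the owner's AC_Inventory reports HasItem and that FlipCooldown has elapsed since LastFlipTime.
; It then records the current game time and calls FlipEra on the object returned by GetTimeLoop.
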(event EventBeginPlay)

(event EventTick
  (params (DeltaSeconds :type Float%20%28single-precision%29)))

(fn UseMirror
  (bind _returnvalue (Utilities|Time|GetGameTimeinSeconds))
  (bind _has (Default|HasItem (Actor|GetComponentbyClass (Components|GetOwner) "/Game/TVV/Blueprints/Components/AC_Inventory.AC_Inventory_C") "/Game/TVV/Data/Items/DA_MirrorOfPassing.DA_MirrorOfPassing"))
  (if _has
    (if (>= (- _returnvalue (Variables|Default|GetLastFlipTime)) (Variables|Default|GetFlipCooldown))
      (Variables|Default|SetLastFlipTime _returnvalue)
      (bind _timeloop (CallFunction|GetTimeLoop))
      (Default|FlipEra _timeloop))))