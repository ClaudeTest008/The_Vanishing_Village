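; Ghost actor component that runs a gameplay-tag state machine: Echo, Distorted, Vengeful, Released.
; Distorted disables AC_Routine and pins the ghost in place to strike nearby players; Vengeful swaps mesh, chases seen or fast-moving players, otherwise patrols ambush points.
; Delayed attacks deal damage or trigger the player's perfect dodge; hits stagger, and death lowers player pressure.
; Interacting releases Distorted or Vengeful ghosts when the time loop holds their weakness knowledge.
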(event Custom|TakeHit
  (params (Damage :type Float%20%28single-precision%29))
  (bind _output_get (Variables|Default|SetHP (- (Variables|Default|GetHP) Damage)))
  (Variables|Default|SetbStaggered true)
  (if (<= _output_get 0.0)
    (CallFunction|Die)
    (else
      (Utilities|FlowControl|RetriggerableDelay 0.5)
      (Variables|Default|SetbStaggered false))))

(event Custom|Die
  (bind _returnvalue (Components|GetOwner))
  (Niagara|SpawnSystematLocation "/Game/Variant_Combat/VFX/NS_Damage.NS_Damage" (Transformation|GetActorLocation _returnvalue))
  (Default|AddPressure (Actor|GetComponentbyClass (Game|Player|GetPlayerPawn 0) "/Game/TVV/Blueprints/Components/AC_Pressure.AC_Pressure_C") -15.0)
  (Actor|DestroyActor _returnvalue))

(event Custom|StartAttackWindup
  (bind _returnvalue (Game|Player|GetPlayerPawn 0))
  (Utilities|FlowControl|RetriggerableDelay 0.4)
  (if (< (Math|Vector|Distance(Vector) (Transformation|GetActorLocation (Components|GetOwner)) (Transformation|GetActorLocation _returnvalue)) 2.4e+02)
    (bind _asbp_player_character (Utilities|Casting|CastToBP_PlayerCharacter _returnvalue))
    (if (Variables|/Game/TVV/Blueprints/Player/BP_PlayerCharacter.BP_PlayerCharacter_C|GetbDodging _asbp_player_character)
      (Default|OnPerfectDodge _asbp_player_character)
      (else
        (Game|Damage|ApplyDamage _returnvalue (Math|Float|SelectFloat 14.0 7.0 (GameplayTags|MatchesTag (Variables|Default|GetCurrentState) "(TagName=\"State.Ghost.Vengeful\")" true)) 0 0)))))

(event EventTick
  (params (DeltaSeconds :type Float%20%28single-precision%29))
  (bind _currentstate (Variables|Default|GetCurrentState))
  (if (GameplayTags|MatchesTag _currentstate "(TagName=\"State.Ghost.Distorted\")" true)
    (CallFunction|TickDistorted)
    (elif (GameplayTags|MatchesTag _currentstate "(TagName=\"State.Ghost.Vengeful\")" true)
      (CallFunction|TickVengeful))))

(fn InitGhost
  (params (Behavior :type Gameplay%20Tag%20Structure) (Speed :type Float%20%28single-precision%29) (MeshPath :type Soft%20Object%20Path%20Structure) (Cry :type Text) (Weakness :type Gameplay%20Tag%20Structure) (Hint :type Text))
  (Variables|Default|SetBehaviorTag Behavior)
  (Variables|Default|SetHuntSpeed Speed)
  (Variables|Default|SetVengefulMeshPath MeshPath)
  (Variables|Default|SetCryText Cry)
  (Variables|Default|SetWeaknessTag Weakness)
  (Variables|Default|SetHintText Hint)
  (Variables|Default|SetCurrentState "(TagName=\"State.Ghost.Echo\")"))

(fn SetGhostState
  (params (NewState :type Gameplay%20Tag%20Structure))
  (bind _returnvalue (Components|GetOwner))
  (bind _returnvalue_2 (Actor|GetComponentbyClass _returnvalue "/Game/TVV/Blueprints/Components/AC_Routine.AC_Routine_C"))
  (Variables|Default|SetCurrentState NewState)
  (Default|CallOnStateChanged NewState)
  (if (GameplayTags|MatchesTag NewState "(TagName=\"State.Ghost.Distorted\")" true)
    (Components|Tick|SetComponentTickEnabled _returnvalue_2 false)
    (Variables|Default|SetHomeLocation (Transformation|GetActorLocation _returnvalue))
    (CallFunction|SetSpeech "...")
    (elif (GameplayTags|MatchesTag NewState "(TagName=\"State.Ghost.Vengeful\")" true)
      (Components|Tick|SetComponentTickEnabled _returnvalue_2 false)
      (bind _returnvalue_3 (Utilities|LoadAssetBlocking (Class|KismetSystemLibrary|ToSoftObjRef(SoftObjPath) (Variables|Default|GetVengefulMeshPath))))
      (bind _asstatic_mesh (Utilities|Casting|CastToStaticMesh _returnvalue_3))
      (Components|StaticMesh|SetStaticMesh (Actor|GetComponentbyClass _returnvalue "/Script/Engine.StaticMeshComponent") _asstatic_mesh)
      (bind _ascharacter (Utilities|Casting|CastToCharacter _returnvalue))
      (Variables|/Script/Engine.CharacterMovementComponent|SetMaxWalkSpeed (Variables|/Script/Engine.Character|GetCharacterMovement _ascharacter) (Variables|Default|GetHuntSpeed))
      (CallFunction|SetSpeech (Variables|Default|GetCryText))
      (bind _ghosts (CallFunction|GetGhosts))
      (bind (_point _found) (Default|GetAmbushPoint _ghosts))
      (Variables|Default|SetPatrolPoint _point)
      (Variables|Default|SetbHasPatrol _found)
      (elif (GameplayTags|MatchesTag NewState "(TagName=\"State.Ghost.Released\")" true)
        (CallFunction|SetSpeech (Variables|Default|GetHintText))
        (bind _ascharacter_2 (Utilities|Casting|CastToCharacter _returnvalue))
        (Variables|/Script/Engine.CharacterMovementComponent|SetMaxWalkSpeed (Variables|/Script/Engine.Character|GetCharacterMovement _ascharacter_2) 1e+02)))))

(fn SetSpeech
  (params (Line :type Text))
  (bind _returnvalue (Components|GetOwner))
  (bind _returnvalue_2 (Actor|GetComponentbyClass _returnvalue "/Script/Engine.TextRenderComponent"))
  (if (Utilities|IsValid _returnvalue_2)
    (Rendering|Components|TextRender|SetText _returnvalue_2 Line)))

(fn TickDistorted
  (bind _returnvalue (Components|GetOwner))
  (bind _returnvalue_2 (Utilities|Time|GetTimeSeconds))
  (Transformation|SetActorLocation _returnvalue (+ (Variables|Default|GetHomeLocation) (* (Math|Random|RandomUnitVector) "")) false false)
  (if (and (< (Math|Vector|Distance(Vector) (Transformation|GetActorLocation _returnvalue) (Transformation|GetActorLocation (Game|Player|GetPlayerPawn 0))) 1.7e+02) (>= _returnvalue_2 (Variables|Default|GetNextAttackTime)))
    (Variables|Default|SetNextAttackTime (+ _returnvalue_2 2.2))
    (CallFunction|StartAttackWindup)))

(fn TickVengeful
  (bind _returnvalue (Components|GetOwner))
  (bind _returnvalue_2 (Game|Player|GetPlayerPawn 0))
  (bind _returnvalue_3 (Utilities|Time|GetTimeSeconds))
  (bind _returnvalue_4 (Transformation|GetActorLocation _returnvalue))
  (bind _returnvalue_5 (Transformation|GetActorLocation _returnvalue_2))
  (bind _returnvalue_6 (Math|Vector|Distance(Vector) _returnvalue_4 _returnvalue_5))
  (if (not (Variables|Default|GetbStaggered))
    (bind _outhit (Collision|LineTraceByChannel _returnvalue_4 _returnvalue_5 "TraceTypeQuery1" false 0 "None"))
    (if (< _returnvalue_6 1.3e+02)
      (if (>= _returnvalue_3 (Variables|Default|GetNextAttackTime))
        (Variables|Default|SetNextAttackTime (+ _returnvalue_3 1.4))
        (CallFunction|StartAttackWindup))
      (elif (or (and (< _returnvalue_6 9e+02) (== (.HitActor (Collision|BreakHitResult _outhit)) _returnvalue_2)) (and (< _returnvalue_6 1.5e+03) (> (Math|Vector|VectorLength (Transformation|GetVelocity _returnvalue_2)) 3e+02)))
        (bind _aspawn (Utilities|Casting|CastToPawn _returnvalue))
        (Pawn|Input|AddMovementInput _aspawn (Math|Vector|GetUnitDirection(Vector) _returnvalue_4 _returnvalue_5) 1.0 false)
        (elif (Variables|Default|GetbHasPatrol)
          (if (< (Math|Vector|Distance2D(Vector) _returnvalue_4 (Variables|Default|GetPatrolPoint)) 1e+02)
            (bind _ghosts (CallFunction|GetGhosts))
            (bind _point (Default|GetAmbushPoint _ghosts))
            (Variables|Default|SetPatrolPoint _point)
            (else
              (bind _aspawn_2 (Utilities|Casting|CastToPawn _returnvalue))
              (Pawn|Input|AddMovementInput _aspawn_2 (Math|Vector|GetUnitDirection(Vector) _returnvalue_4 (Variables|Default|GetPatrolPoint)) 1.0 false))))))))

(fn HandleInteract
  (bind _currentstate (Variables|Default|GetCurrentState))
  (bind _timeloop (CallFunction|GetTimeLoop))
  (bind _has (Default|HasKnowledge _timeloop (Variables|Default|GetWeaknessTag)))
  (if (and _has (not (or (GameplayTags|MatchesTag _currentstate "(TagName=\"State.Ghost.Echo\")" true) (GameplayTags|MatchesTag _currentstate "(TagName=\"State.Ghost.Released\")" true))))
    (CallFunction|SetGhostState "(TagName=\"State.Ghost.Released\")")))