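; AC_Routine is an actor component that moves its owning pawn through a timed routine of stops tied to the time loop.
; SetStops supplies parallel arrays of locations and loop-progress fractions.
; Each tick before midnight, it selects the last listed stop whose fraction the elapsed loop progress has reached.
; It steers straight toward that stop with movement input, without pathfinding, until within a small 2D radius.
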(event EventTick
  (params (DeltaSeconds :type Float%20%28single-precision%29))
  (bind _returnvalue (Components|GetOwner))
  (bind _returnvalue_2 (Transformation|GetActorLocation _returnvalue))
  (bind _timeloop (CallFunction|GetTimeLoop))
  (if (Utilities|IsValid _timeloop)
    (if (not (Variables|/Game/TVV/Blueprints/Core/Subsystems/BPS_TimeLoopSubsystem.BPS_TimeLoopSubsystem_C|GetbIsAfterMidnight _timeloop))
      (Variables|Default|SetBestIndex -1)
      (for (_array_element _array_index) (Variables|Default|GetStopFractions)
        (if (<= _array_element (/ (- (Variables|/Game/TVV/Blueprints/Core/Subsystems/BPS_TimeLoopSubsystem.BPS_TimeLoopSubsystem_C|GetLoopDuration _timeloop) (Variables|/Game/TVV/Blueprints/Core/Subsystems/BPS_TimeLoopSubsystem.BPS_TimeLoopSubsystem_C|GetLoopTimeRemaining _timeloop)) (Variables|/Game/TVV/Blueprints/Core/Subsystems/BPS_TimeLoopSubsystem.BPS_TimeLoopSubsystem_C|GetLoopDuration _timeloop)))
          (Variables|Default|SetBestIndex _array_index)))
      (if (>= (Variables|Default|GetBestIndex) 0)
        (Variables|Default|SetCurrentIndex (Variables|Default|GetBestIndex))
        (bind _aspawn (Utilities|Casting|CastToPawn _returnvalue))
        (if (> (Math|Vector|Distance2D(Vector) _returnvalue_2 (Utilities|Array|Get(acopy) (Variables|Default|GetStopLocations) (Variables|Default|GetBestIndex))) 8e+01)
          (Pawn|Input|AddMovementInput _aspawn (Math|Vector|GetUnitDirection(Vector) _returnvalue_2 (Utilities|Array|Get(acopy) (Variables|Default|GetStopLocations) (Variables|Default|GetBestIndex))) 1.0 false))))))

(fn SetStops
  (params (Locations :type Array%20of%20Vectors) (Fractions :type Array%20of%20Floats%20%28single-precision%29))
  (Variables|Default|SetStopLocations Locations)
  (Variables|Default|SetStopFractions Fractions)
  (Variables|Default|SetCurrentIndex -1))