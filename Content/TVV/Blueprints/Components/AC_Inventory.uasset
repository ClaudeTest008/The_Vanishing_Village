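; Inventory component that stores items as stacked entries, matched by the soft reference path of each item.
; Add and remove adjust or delete stacks and broadcast OnInventoryChanged, with helpers for count, presence and contents queries.
; Using an item consumes one and fires OnItemUsed, while examining only fires OnItemExamined.
; ResetForLoop blocking-loads each PDA_Item and keeps only those flagged PersistentThroughLoops.
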(event EventBeginPlay)

(event EventTick
  (params (DeltaSeconds :type Float%20%28single-precision%29)))

(fn FindItemIndex
  (params (Item :type Soft%20Object%20Path%20Structure))
  (LocalVariables|SetFoundIndex -1)
  (for (_array_element _array_index) (Variables|Default|GetItems)
    (if (Utilities|Enum|Equal(Enum) (Utilities|BreakSoftObjectPath (.Item (Utilities|Struct|BreakFInventoryEntry _array_element))) (Utilities|BreakSoftObjectPath Item))
      (LocalVariables|SetFoundIndex _array_index)))
  (return (LocalVariables|GetFoundIndex)))

(fn AddItem
  (params (Item :type Soft%20Object%20Path%20Structure) (Count :type Integer))
  (bind _index (CallFunction|FindItemIndex Item))
  (if (>= _index 0)
    (Utilities|Array|SetArrayElem (Variables|Default|GetItems) _index (Utilities|Struct|MakeFInventoryEntry (+ (.StackCount (Utilities|Struct|BreakFInventoryEntry (Utilities|Array|Get(acopy) (Variables|Default|GetItems) _index))) Count) Item))
    (else
      (Utilities|Array|Add (Variables|Default|GetItems) (Utilities|Struct|MakeFInventoryEntry Count Item))))
  (Default|CallOnInventoryChanged)
  (return true))

(fn RemoveItem
  (params (Item :type Soft%20Object%20Path%20Structure) (Count :type Integer))
  (bind _index (CallFunction|FindItemIndex Item))
  (if (>= _index 0)
    (if (<= (- (.StackCount (Utilities|Struct|BreakFInventoryEntry (Utilities|Array|Get(acopy) (Variables|Default|GetItems) _index))) Count) 0)
      (Utilities|Array|RemoveIndex (Variables|Default|GetItems) _index)
      (else
        (Utilities|Array|SetArrayElem (Variables|Default|GetItems) _index (Utilities|Struct|MakeFInventoryEntry (- (.StackCount (Utilities|Struct|BreakFInventoryEntry (Utilities|Array|Get(acopy) (Variables|Default|GetItems) _index))) Count) Item))))
    (Default|CallOnInventoryChanged)
    (return true)
    (else
      (return false))))

(fn GetItemCount
  (params (Item :type Soft%20Object%20Path%20Structure))
  (bind _index (CallFunction|FindItemIndex Item))
  (if (>= _index 0)
    (return (.StackCount (Utilities|Struct|BreakFInventoryEntry (Utilities|Array|Get(acopy) (Variables|Default|GetItems) _index))))
    (else
      (return 0))))

(fn HasItem
  (params (Item :type Soft%20Object%20Path%20Structure))
  (bind _count (CallFunction|GetItemCount Item))
  (return (> _count 0)))

(fn GetInventoryContents
  (return (Variables|Default|GetItems)))

(fn UseItem
  (params (Item :type Soft%20Object%20Path%20Structure))
  (bind _success (CallFunction|RemoveItem Item 1))
  (if _success
    (Default|CallOnItemUsed Item)))

(fn ExamineItem
  (params (Item :type Soft%20Object%20Path%20Structure))
  (Default|CallOnItemExamined Item))

(fn ResetforLoop
  (for _array_element (Variables|Default|GetItems)
    (bind _returnvalue (Utilities|LoadAssetBlocking (Class|KismetSystemLibrary|ToSoftObjRef(SoftObjPath) (.Item (Utilities|Struct|BreakFInventoryEntry _array_element)))))
    (bind _aspda_item (Utilities|Casting|CastToPDA_Item _returnvalue))
    (if (Variables|/Game/TVV/Data/Definitions/PDA_Item.PDA_Item_C|GetbPersistentThroughLoops _aspda_item)
      (Utilities|Array|Add (LocalVariables|GetKept) _array_element)))
  (Variables|Default|SetItems (LocalVariables|GetKept))
  (Default|CallOnInventoryChanged))