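; Interaction component that detects what the player camera looks at and lets its owner interact with or examine it.
; Each tick, a Visibility line trace from the camera caches the hit actor's AC_Interactable and broadcasts prompt show or hide when the target changes.
; TryInteract triggers the cached interactable, while ExamineCurrent passes its AC_InventoryItemMarker item to the owner's AC_Inventory.
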(event EventTick
  (params (DeltaSeconds :type Float%20%28single-precision%29))
  (bind _returnvalue (Game|GetPlayerCameraManager 0))
  (bind _returnvalue_2 (Camera|GetCameraLocation _returnvalue))
  (bind _outhit (Collision|LineTraceByChannel _returnvalue_2 (+ _returnvalue_2 (* (Transformation|GetActorForwardVector _returnvalue) (Variables|Default|GetTraceDistance))) "TraceTypeQuery1" false 0 "None"))
  (if (Utilities|IsValid (.HitActor (Collision|BreakHitResult _outhit)))
    (if (!= (Actor|GetComponentbyClass (.HitActor (Collision|BreakHitResult _outhit)) "/Game/TVV/Blueprints/Components/AC_Interactable.AC_Interactable_C") (Variables|Default|GetCurrentInteractable))
      (Variables|Default|SetCurrentInteractable (Actor|GetComponentbyClass (.HitActor (Collision|BreakHitResult _outhit)) "/Game/TVV/Blueprints/Components/AC_Interactable.AC_Interactable_C"))
      (if (Utilities|IsValid (Actor|GetComponentbyClass (.HitActor (Collision|BreakHitResult _outhit)) "/Game/TVV/Blueprints/Components/AC_Interactable.AC_Interactable_C")) :!label _label
        (Default|CallOnInteractableChanged (Variables|/Game/TVV/Blueprints/Components/AC_Interactable.AC_Interactable_C|GetPromptText (Actor|GetComponentbyClass (.HitActor (Collision|BreakHitResult _outhit)) "/Game/TVV/Blueprints/Components/AC_Interactable.AC_Interactable_C")) true)
        (else
          (Default|CallOnInteractableChanged "" false))))
    (elif (Utilities|IsValid (Variables|Default|GetCurrentInteractable))
      (Variables|Default|SetCurrentInteractable 0)
      (goto _label))))

(fn TryInteract
  (bind _currentinteractable (Variables|Default|GetCurrentInteractable))
  (if (Utilities|IsValid _currentinteractable)
    (Default|OnInteracted _currentinteractable)))

(fn ExamineCurrent
  (bind _currentinteractable (Variables|Default|GetCurrentInteractable))
  (bind _returnvalue (Components|GetOwner _currentinteractable))
  (bind _returnvalue_2 (Actor|GetComponentbyClass _returnvalue "/Game/TVV/Blueprints/Components/AC_InventoryItemMarker.AC_InventoryItemMarker_C"))
  (if (Utilities|IsValid _currentinteractable)
    (if (Utilities|IsValid _returnvalue_2)
      (Default|ExamineItem (Actor|GetComponentbyClass (Components|GetOwner) "/Game/TVV/Blueprints/Components/AC_Inventory.AC_Inventory_C") (Variables|/Game/TVV/Blueprints/Components/AC_InventoryItemMarker.AC_InventoryItemMarker_C|GetItem _returnvalue_2)))))