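; Actor component that tracks a 0–100 Pressure meter on its owner and turns it into escalating sensory effects.
; Each tick, time of night and the nearest vengeful villager ghost feed Pressure, while unlocking knowledge in the time loop relieves it.
; Pressure scales camera pitch sway, post-process blend and crossfaded 2D ambience layers, which also switch at midnight.
; Above a threshold, it periodically spawns echo-figure hallucinations near the owner.
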(event Custom|HandleKnowledge
  (params (Tag :type Gameplay%20Tag%20Structure))
  (CallFunction|AddPressure -1e+01))

(event EventBeginPlay
  (CallFunction|StartAmbience)
  (bind _timeloop (CallFunction|GetTimeLoop))
  (EventDispatchers|BindEventtoOnKnowledgeUnlocked _timeloop (delegate Custom|HandleKnowledge)))

(event EventTick
  (params (DeltaSeconds :type Float%20%28single-precision%29))
  (CallFunction|TickSources DeltaSeconds)
  (CallFunction|TickEffects DeltaSeconds)
  (CallFunction|UpdateAmbience))

(fn AddPressure
  (params (Amount :type Float%20%28single-precision%29))
  (Variables|Default|SetPressure (Math|Float|Clamp(Float) (+ (Variables|Default|GetPressure) Amount) 0.0 1e+02)))

(fn StartAmbience
  (bind _returnvalue (Audio|SpawnSound2D "/Game/ENTROPYSTARTER/WAVS/WAV_after_hours.WAV_after_hours" 0.8 1.0 0.0 0))
  (Variables|Default|SetAmbDay _returnvalue)
  (bind _returnvalue_2 (Audio|SpawnSound2D "/Game/ENTROPYSTARTER/WAVS/WAV_deja_vu.WAV_deja_vu" 0.0 1.0 0.0 0))
  (Variables|Default|SetAmbNight _returnvalue_2)
  (bind _returnvalue_3 (Audio|SpawnSound2D "/Game/ENTROPYSTARTER/WAVS/WAV_echoes.WAV_echoes" 0.0 1.0 0.0 0))
  (Variables|Default|SetAmbLow _returnvalue_3)
  (bind _returnvalue_4 (Audio|SpawnSound2D "/Game/ENTROPYSTARTER/WAVS/WAV_internal_monologue.WAV_internal_monologue" 0.0 1.0 0.0 0))
  (Variables|Default|SetAmbMid _returnvalue_4)
  (bind _returnvalue_5 (Audio|SpawnSound2D "/Game/ENTROPYSTARTER/WAVS/WAV_simulation.WAV_simulation" 0.0 1.0 0.0 0))
  (Variables|Default|SetAmbHigh _returnvalue_5))

(fn UpdateAmbience
  (bind _pressure (Variables|Default|GetPressure))
  (bind _ambday (Variables|Default|GetAmbDay))
  (bind _ambnight (Variables|Default|GetAmbNight))
  (bind _amblow (Variables|Default|GetAmbLow))
  (bind _ambmid (Variables|Default|GetAmbMid))
  (bind _ambhigh (Variables|Default|GetAmbHigh))
  (bind _timeloop (CallFunction|GetTimeLoop))
  (if (Utilities|IsValid _ambday)
    (Audio|Components|Audio|SetVolumeMultiplier _ambday (Math|Float|SelectFloat 0.0 (Math|Float|MapRangeClamped _pressure 0.0 1.5e+02 0.8 0.0) (Variables|/Game/TVV/Blueprints/Core/Subsystems/BPS_TimeLoopSubsystem.BPS_TimeLoopSubsystem_C|GetbIsAfterMidnight _timeloop)) :!class /Script/Engine.AudioComponent)
    (if (Utilities|IsValid _ambnight)
      (Audio|Components|Audio|SetVolumeMultiplier _ambnight (Math|Float|SelectFloat 0.6 0.0 (Variables|/Game/TVV/Blueprints/Core/Subsystems/BPS_TimeLoopSubsystem.BPS_TimeLoopSubsystem_C|GetbIsAfterMidnight _timeloop)) :!class /Script/Engine.AudioComponent)
      (if (Utilities|IsValid _amblow)
        (Audio|Components|Audio|SetVolumeMultiplier _amblow (Math|Float|MapRangeClamped _pressure 3e+01 1e+02 0.0 0.7) :!class /Script/Engine.AudioComponent)
        (if (Utilities|IsValid _ambmid)
          (Audio|Components|Audio|SetVolumeMultiplier _ambmid (Math|Float|MapRangeClamped _pressure 6e+01 1e+02 0.0 0.8) :!class /Script/Engine.AudioComponent)
          (if (Utilities|IsValid _ambhigh)
            (Audio|Components|Audio|SetVolumeMultiplier _ambhigh (Math|Float|MapRangeClamped _pressure 8e+01 1e+02 0.0 0.9) :!class /Script/Engine.AudioComponent)))))))

(fn TriggerHallucination
  (bind _returnvalue (Components|GetOwner))
  (bind _returnvalue_2 (Math|Random|RandomUnitVector))
  (bind _returnvalue_3 (Transformation|GetActorLocation _returnvalue))
  (bind _returnvalue_4 (* _returnvalue_2 ""))
  (bind _returnvalue_5 (* _returnvalue_4 "(X=1.0,Y=1.0,Z=0.0)"))
  (bind _returnvalue_6 (+ _returnvalue_3 _returnvalue_5))
  (bind _returnvalue_7 (Game|SpawnActorfromClass "/Game/TVV/Blueprints/World/BP_EchoFigure.BP_EchoFigure_C" (Math|Transform|MakeTransform _returnvalue_6) "AlwaysSpawn" "MultiplyWithRoot" 0 0))
  (Default|PlayScene _returnvalue_7 _returnvalue_6 (+ _returnvalue_6 "(X=120.0,Y=0.0,Z=0.0)") "" "" 4.0)
  (if (>= (Variables|Default|GetPressure) (Variables|Default|GetThresholdHigh))
    (bind _returnvalue_8 (Actor|GetActorOfClass "/Game/TVV/Blueprints/World/BP_Pickup_Base.BP_Pickup_Base_C"))
    (if (Utilities|IsValid _returnvalue_8)
      (Transformation|AddActorLocalRotation _returnvalue_8 "0, 0, 0" false false))))

(fn TickSources
  (params (Delta :type Float%20%28single-precision%29))
  (bind _returnvalue (Components|GetOwner))
  (bind _returnvalue_2 (Transformation|GetActorLocation _returnvalue))
  (bind _timeloop (CallFunction|GetTimeLoop))
  (CallFunction|AddPressure (* (Math|Float|SelectFloat 2.0 (Math|Float|SelectFloat 0.5 -0.5 (Variables|/Game/TVV/Blueprints/Core/Subsystems/BPS_TimeLoopSubsystem.BPS_TimeLoopSubsystem_C|GetbMidnightWarned _timeloop)) (Variables|/Game/TVV/Blueprints/Core/Subsystems/BPS_TimeLoopSubsystem.BPS_TimeLoopSubsystem_C|GetbIsAfterMidnight _timeloop)) Delta))
  (LocalVariables|SetMinDist 1e+05)
  (bind _outactors (Actor|GetAllActorsOfClass "/Game/TVV/Blueprints/World/BP_Villager_Base.BP_Villager_Base_C"))
  (for _array_element _outactors
    (if (and (GameplayTags|MatchesTag (Variables|/Game/TVV/Blueprints/Components/AC_Ghost.AC_Ghost_C|GetCurrentState (Actor|GetComponentbyClass _array_element "/Game/TVV/Blueprints/Components/AC_Ghost.AC_Ghost_C")) "(TagName=\"State.Ghost.Vengeful\")" true) (< (Math|Vector|Distance(Vector) _returnvalue_2 (Transformation|GetActorLocation _array_element)) (LocalVariables|GetMinDist)))
      (LocalVariables|SetMinDist (Math|Vector|Distance(Vector) _returnvalue_2 (Transformation|GetActorLocation _array_element)))))
  (CallFunction|AddPressure (* (Math|Float|MapRangeClamped (LocalVariables|GetMinDist) 0.0 8e+02 4.0 0.0) Delta))
  (bind _returnvalue_3 (Actor|GetActorOfClass "/Game/TVV/Blueprints/World/BP_TimeMachine.BP_TimeMachine_C"))
  (if (< (Math|Vector|Distance(Vector) _returnvalue_2 (Transformation|GetActorLocation _returnvalue_3)) 6e+02)
    (CallFunction|AddPressure (* 0.0 Delta))))

(fn TickEffects
  (params (Delta :type Float%20%28single-precision%29))
  (bind _pressure (Variables|Default|GetPressure))
  (bind _output_get (Variables|Default|SetBreathPhase (+ (Variables|Default|GetBreathPhase) (* 0.0 Delta))))
  (bind _aspawn (Utilities|Casting|CastToPawn (Components|GetOwner)))
  (Pawn|Input|AddControllerPitchInput _aspawn (* (Math|Trig|Sin(Radians) _output_get) (Math|Float|MapRangeClamped _pressure 3e+01 1e+02 0.0 0.05)))
  (bind _returnvalue (Actor|GetActorOfClass "/Script/Engine.PostProcessVolume"))
  (if (Utilities|IsValid _returnvalue)
    (Variables|/Script/Engine.PostProcessVolume|SetBlendWeight _returnvalue (Math|Float|MapRangeClamped _pressure 2e+01 1e+02 0.0 1.0)))
  (bind _output_get_2 (Variables|Default|SetHallucinationAccum (+ (Variables|Default|GetHallucinationAccum) Delta)))
  (if (and (> _output_get_2 1e+01) (>= _pressure (Variables|Default|GetThresholdMid)))
    (Variables|Default|SetHallucinationAccum 0.0)
    (CallFunction|TriggerHallucination)))