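; BP_VillageDirector populates the village with residents and drives their ghost states in step with the time loop.
; It spawns a BP_Villager_Base for each DT_Residents row at the origin, then initializes it with that row's resident data.
; Time loop events trigger a full despawn and respawn on loop start or a flip away from the present.
; Approaching midnight sets all villagers' AC_Ghost to Distorted, while midnight or flipping to the present sets Vengeful.
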(event Custom|HandleLoopStarted
  (params (LoopNumber :type Integer))
  (CallFunction|DespawnAll)
  (CallFunction|SpawnAll))

(event Custom|HandleMidnight
  (CallFunction|SetAllGhostStates "(TagName=\"State.Ghost.Vengeful\")"))

(event Custom|HandleApproaching
  (CallFunction|SetAllGhostStates "(TagName=\"State.Ghost.Distorted\")"))

(event Custom|HandleEraFlip
  (params (bToPresent :type Boolean))
  (if bToPresent
    (CallFunction|SetAllGhostStates "(TagName=\"State.Ghost.Vengeful\")")
    (else
      (CallFunction|DespawnAll)
      (CallFunction|SpawnAll))))

(event EventBeginPlay
  (CallFunction|SpawnAll)
  (bind _timeloop (CallFunction|GetTimeLoop))
  (EventDispatchers|BindEventtoOnLoopStarted _timeloop (delegate Custom|HandleLoopStarted))
  (EventDispatchers|BindEventtoOnMidnightTriggered _timeloop (delegate Custom|HandleMidnight))
  (EventDispatchers|BindEventtoOnMidnightApproaching _timeloop (delegate Custom|HandleApproaching))
  (EventDispatchers|BindEventtoOnEraFlipped _timeloop (delegate Custom|HandleEraFlip)))

(fn ConstructionScript)

(fn SpawnAll
  (bind _outrownames (DataTable|GetDataTableRowNames "/Game/TVV/Data/DT_Residents.DT_Residents"))
  (for _array_element _outrownames
    (bind _returnvalue (Utilities|GetDataTableRow "/Game/TVV/Data/DT_Residents.DT_Residents" _array_element)
      (:then
        (bind _returnvalue_2 (Game|SpawnActorfromClass "/Game/TVV/Blueprints/World/BP_Villager_Base.BP_Villager_Base_C" (Math|Transform|MakeTransform "0, 0, 0") "AlwaysSpawn" "MultiplyWithRoot" 0 0))
        (Default|InitResident _returnvalue_2 (Utilities|Struct|BreakFResidentRow _returnvalue))))))

(fn DespawnAll
  (bind _outactors (Actor|GetAllActorsOfClass "/Game/TVV/Blueprints/World/BP_Villager_Base.BP_Villager_Base_C"))
  (for _array_element _outactors
    (Actor|DestroyActor _array_element)))

(fn SetAllGhostStates
  (params (State :type Gameplay%20Tag%20Structure))
  (bind _outactors (Actor|GetAllActorsOfClass "/Game/TVV/Blueprints/World/BP_Villager_Base.BP_Villager_Base_C"))
  (for _array_element _outactors
    (Default|SetGhostState (Actor|GetComponentbyClass _array_element "/Game/TVV/Blueprints/Components/AC_Ghost.AC_Ghost_C") State)))