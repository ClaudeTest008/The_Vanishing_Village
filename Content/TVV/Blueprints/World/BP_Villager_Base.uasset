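; BP_Villager_Base is a base villager actor configured from a resident data asset, with an observe prompt and ghost behavior.
; InitResident blocking-loads the PDA_Resident and its mesh, sets up the Figure and prompt, feeds routine stops to Routine, and moves the actor just above the first stop.
; It also passes behavior, hunt speed, vengeful mesh and cry, weakness and hint to Ghost, which handles every interaction.
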(event OnInteract(Interactable)
  (Default|HandleInteract (Variables|Default|GetGhost)))

(event EventBeginPlay)

(event Collision|EventActorBeginOverlap
  (params (OtherActor :type Actor%20Object%20Reference)))

(event EventTick
  (params (DeltaSeconds :type Float%20%28single-precision%29)))

(fn ConstructionScript)

(fn InitResident
  (params (ResidentPath :type Soft%20Object%20Path%20Structure))
  (Variables|Default|SetResidentDef ResidentPath)
  (bind _returnvalue (Utilities|LoadAssetBlocking (Class|KismetSystemLibrary|ToSoftObjRef(SoftObjPath) ResidentPath)))
  (bind _aspda_resident (Utilities|Casting|CastToPDA_Resident _returnvalue))
  (bind _returnvalue_2 (Utilities|LoadAssetBlocking (Class|KismetSystemLibrary|ToSoftObjRef(SoftObjPath) (Variables|/Game/TVV/Data/Definitions/PDA_Resident.PDA_Resident_C|GetFigureMesh _aspda_resident))))
  (bind _asstatic_mesh (Utilities|Casting|CastToStaticMesh _returnvalue_2))
  (Components|StaticMesh|SetStaticMesh (Variables|Default|GetFigure) _asstatic_mesh)
  (Transformation|SetRelativeScale3D (Variables|Default|GetFigure) (Math|Conversions|ToVector(Float) (Variables|/Game/TVV/Data/Definitions/PDA_Resident.PDA_Resident_C|GetFigureScale _aspda_resident)))
  (Variables|/Game/TVV/Blueprints/Components/AC_Interactable.AC_Interactable_C|SetPromptText (Variables|Default|GetInteractable) (Utilities|Text|ToText(String) (Utilities|String|Append "Observe " (Utilities|String|ToString(Text) (Variables|/Game/TVV/Data/Definitions/PDA_Resident.PDA_Resident_C|GetDisplayName _aspda_resident)))))
  (Default|SetStops (Variables|Default|GetRoutine) (Variables|/Game/TVV/Data/Definitions/PDA_Resident.PDA_Resident_C|GetRoutineLocations _aspda_resident) (Variables|/Game/TVV/Data/Definitions/PDA_Resident.PDA_Resident_C|GetRoutineFractions _aspda_resident))
  (Transformation|SetActorLocation (+ (Utilities|Array|Get(acopy) (Variables|/Game/TVV/Data/Definitions/PDA_Resident.PDA_Resident_C|GetRoutineLocations _aspda_resident)) "(X=0,Y=0,Z=100)") false false)
  (Default|InitGhost (Variables|Default|GetGhost) (Variables|/Game/TVV/Data/Definitions/PDA_Resident.PDA_Resident_C|GetGhostBehaviorTag _aspda_resident) (Variables|/Game/TVV/Data/Definitions/PDA_Resident.PDA_Resident_C|GetGhostHuntSpeed _aspda_resident) (Variables|/Game/TVV/Data/Definitions/PDA_Resident.PDA_Resident_C|GetVengefulMeshPath _aspda_resident) (Variables|/Game/TVV/Data/Definitions/PDA_Resident.PDA_Resident_C|GetVengefulCry _aspda_resident) (Variables|/Game/TVV/Data/Definitions/PDA_Resident.PDA_Resident_C|GetWeakness _aspda_resident) (Variables|/Game/TVV/Data/Definitions/PDA_Resident.PDA_Resident_C|GetReleasedHint _aspda_resident)))