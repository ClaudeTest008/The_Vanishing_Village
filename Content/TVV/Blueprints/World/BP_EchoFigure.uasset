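; BP_EchoFigure is an actor that plays a short scripted scene as a figure with floating speech text, then destroys itself.
; On BeginPlay it synchronously loads a static mesh from a path and assigns it to the figure.
; PlayScene stores endpoints, two lines and a duration, then shows the first line.
; Tick linearly moves it between the points by elapsed game time, switching to the second line past halfway.
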(event EventTick
  (params (DeltaSeconds :type Float%20%28single-precision%29))
  (bind _returnvalue (Utilities|Time|GetGameTimeinSeconds))
  (bind _starttime (Variables|Default|GetStartTime))
  (bind _sceneduration (Variables|Default|GetSceneDuration))
  (bind _returnvalue_2 (- _returnvalue _starttime))
  (bind _returnvalue_3 (/ _returnvalue_2 _sceneduration))
  (if (Variables|Default|GetbPlaying)
    (if (>= _returnvalue_3 1.0)
      (Actor|DestroyActor)
      (else
        (Transformation|SetActorLocation (Math|Vector|Lerp(Vector) (Variables|Default|GetPStart) (Variables|Default|GetPEnd) _returnvalue_3) false false)
        (if (> _returnvalue_3 0.5)
          (Rendering|Components|TextRender|SetText (Variables|Default|GetSpeechText) (Variables|Default|GetLine2)))))))

(event EventBeginPlay
  (bind _returnvalue (Utilities|LoadAssetBlocking (Class|KismetSystemLibrary|ToSoftObjRef(SoftObjPath) (Variables|Default|GetMeshPath))))
  (bind _asstatic_mesh (Utilities|Casting|CastToStaticMesh _returnvalue))
  (Components|StaticMesh|SetStaticMesh (Variables|Default|GetFigure) _asstatic_mesh))

(fn ConstructionScript)

(fn PlayScene
  (params (Start :type Vector) (End :type Vector) (L1 :type Text) (L2 :type Text) (Duration :type Float%20%28single-precision%29))
  (Variables|Default|SetPStart Start)
  (Variables|Default|SetPEnd End)
  (Variables|Default|SetLine1 L1)
  (Variables|Default|SetLine2 L2)
  (Variables|Default|SetSceneDuration Duration)
  (Variables|Default|SetStartTime (Utilities|Time|GetGameTimeinSeconds))
  (Variables|Default|SetbPlaying true)
  (Transformation|SetActorLocation Start false false)
  (Rendering|Components|TextRender|SetText (Variables|Default|GetSpeechText) L1))