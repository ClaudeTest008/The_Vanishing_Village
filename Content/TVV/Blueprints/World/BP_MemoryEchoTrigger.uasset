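; Interactable shimmer that replays a memory echo of a market quarrel over debt between Aiko and Ichiro in a time-loop game.
; With the quarrel clue known and before midnight, interacting spawns two BP_EchoFigure actors at hardcoded positions to play the scene, then immediately unlocks the merchant debt knowledge.
; It plays once per loop, resetting on the time loop's start event.
; BeginPlay also blocking-loads the shimmer mesh from a path.
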(event OnInteract(Interactable)
  (bind _timeloop (CallFunction|GetTimeLoop))
  (bind _has (Default|HasKnowledge _timeloop "(TagName=\"Knowledge.Clue.MarketQuarrel\")"))
  (if (and (and _has (not (Variables|/Game/TVV/Blueprints/Core/Subsystems/BPS_TimeLoopSubsystem.BPS_TimeLoopSubsystem_C|GetbIsAfterMidnight _timeloop))) (not (Variables|Default|GetbPlayed)))
    (Variables|Default|SetbPlayed true)
    (bind _returnvalue (Game|SpawnActorfromClass "/Game/TVV/Blueprints/World/BP_EchoFigure.BP_EchoFigure_C" (Math|Transform|MakeTransform "(X=100,Y=900,Z=90)") "Undefined" "MultiplyWithRoot" 0 0))
    (Default|PlayScene _returnvalue "(X=100,Y=900,Z=90)" "(X=280,Y=960,Z=90)" "You still owe for the winter rice, Aiko." "The ledger does not forget. Neither do I." 4e+01)
    (bind _returnvalue_2 (Game|SpawnActorfromClass "/Game/TVV/Blueprints/World/BP_EchoFigure.BP_EchoFigure_C" (Math|Transform|MakeTransform "(X=180,Y=780,Z=90)") "Undefined" "MultiplyWithRoot" 0 0))
    (Default|PlayScene _returnvalue_2 "(X=180,Y=780,Z=90)" "(X=40,Y=840,Z=90)" "My children starve while you count coins, Ichiro." "By dawn the whole village will know what you did." 4e+01)
    (Default|UnlockKnowledge _timeloop "(TagName=\"Knowledge.Resident.MerchantDebt\")")))

(event Custom|HandleLoopStarted
  (params (LoopNumber :type Integer))
  (Variables|Default|SetbPlayed false))

(event EventBeginPlay
  (bind _timeloop (CallFunction|GetTimeLoop))
  (EventDispatchers|BindEventtoOnLoopStarted _timeloop (delegate Custom|HandleLoopStarted))
  (bind _returnvalue (Utilities|LoadAssetBlocking (Class|KismetSystemLibrary|ToSoftObjRef(SoftObjPath) (Variables|Default|GetMeshPath))))
  (bind _asstatic_mesh (Utilities|Casting|CastToStaticMesh _returnvalue))
  (Components|StaticMesh|SetStaticMesh (Variables|Default|GetShimmer) _asstatic_mesh))

(fn ConstructionScript)