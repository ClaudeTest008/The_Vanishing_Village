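; Base world pickup actor that the player interacts with to collect the item and count set on its ItemMarker.
; On BeginPlay it synchronously loads the PDA_Item data asset and builds the Interactable prompt from its display name.
; On interact it adds the item to the player pawn's AC_Inventory.
; If that succeeds, it unlocks any valid knowledge tag through the time loop and destroys itself.
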(event OnInteract(Interactable)
  (bind _success (Default|AddItem (Actor|GetComponentbyClass (Game|Player|GetPlayerPawn 0) "/Game/TVV/Blueprints/Components/AC_Inventory.AC_Inventory_C") (Variables|/Game/TVV/Blueprints/Components/AC_InventoryItemMarker.AC_InventoryItemMarker_C|GetItem (Variables|Default|GetItemMarker)) (Variables|/Game/TVV/Blueprints/Components/AC_InventoryItemMarker.AC_InventoryItemMarker_C|GetCount (Variables|Default|GetItemMarker))))
  (if _success
    (bind _returnvalue (Utilities|LoadAssetBlocking (Class|KismetSystemLibrary|ToSoftObjRef(SoftObjPath) (Variables|/Game/TVV/Blueprints/Components/AC_InventoryItemMarker.AC_InventoryItemMarker_C|GetItem (Variables|Default|GetItemMarker)))))
    (bind _aspda_item (Utilities|Casting|CastToPDA_Item _returnvalue))
    (if (GameplayTags|IsGameplayTagValid (Variables|/Game/TVV/Data/Definitions/PDA_Item.PDA_Item_C|GetKnowledgeTag _aspda_item))
      (bind _timeloop (CallFunction|GetTimeLoop))
      (Default|UnlockKnowledge _timeloop (Variables|/Game/TVV/Data/Definitions/PDA_Item.PDA_Item_C|GetKnowledgeTag _aspda_item)))
    (Actor|DestroyActor)))

(event EventBeginPlay
  (bind _returnvalue (Utilities|LoadAssetBlocking (Class|KismetSystemLibrary|ToSoftObjRef(SoftObjPath) (Variables|/Game/TVV/Blueprints/Components/AC_InventoryItemMarker.AC_InventoryItemMarker_C|GetItem (Variables|Default|GetItemMarker)))))
  (bind _aspda_item (Utilities|Casting|CastToPDA_Item _returnvalue))
  (Variables|/Game/TVV/Blueprints/Components/AC_Interactable.AC_Interactable_C|SetPromptText (Variables|Default|GetInteractable) (Utilities|Text|ToText(String) (Utilities|String|Append "Pick up " (Utilities|String|ToString(Text) (Variables|/Game/TVV/Data/Definitions/PDA_Item.PDA_Item_C|GetDisplayName _aspda_item))))))

(fn ConstructionScript)